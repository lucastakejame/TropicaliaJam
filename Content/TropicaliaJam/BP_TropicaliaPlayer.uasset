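; BP_TropicaliaPlayer represents a player in the Tropicalia jam card game and manages that player's on-screen hand.
; On BeginPlay it creates a WBP_CardHand widget for its owning PlayerController and adds it to the viewport.
; AddCard forwards single cards to the widget.
; AddCardsToHand, StartTurn and GetHandPileSize are stubs: an empty loop, an empty body and a constant zero.
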(event EventBeginPlay
  (bind _returnvalue (UserInterface|CreateWidget "/Game/TropicaliaJam/WBP_CardHand.WBP_CardHand_C" (.AsPlayer%20Controller (Utilities|Casting|CastToPlayerController (Components|GetOwner)))))
  (bind _output_get (Variables|Default|SetCardHand _returnvalue))
  (UserInterface|Viewport|AddtoViewport _output_get 0)
  (CallFunction|AddCardstoHand (Utilities|Array|MakeArray)))

(fn ConstructionScript)

(fn AddCardstoHand
  (params (Cards :type Array%20of%20BP%20Card%20Object%20References))
  (for _array_element Cards
    _))

(fn StartTurn)

(fn GetHandPileSize
  (return 0))

(fn AddCard
  (params (Card :type BP%20Card%20Object%20Reference))
  (Default|AddCardtoHand (Variables|Default|GetCardHand) Card))