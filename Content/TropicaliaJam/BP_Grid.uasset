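; BP_Grid is the game manager for a turn-based card game, spawning a clickable cell grid and a card pile.
; Each turn tops the active player's hand up to five, with handlers for draw completion and turn end driving the loop.
; Clicking a cell sets its tension.
; Player selection always returns the first player, grid updating is an empty stub, and the game-end check never reports a win or loss.
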(event Custom|OnClicked_Event
  (params (TouchedActor :type Actor%20Object%20Reference) (ButtonPressed :type Key%20Structure :default "None"))
  (bind _asbp_grid_cell (Utilities|Casting|CastToBP_GridCell TouchedActor))
  (Default|SetTension _asbp_grid_cell 1.0))

(event Custom|ExecuteTurn
  (bind _activeplayer (CallFunction|SelectActivePlayer))
  (bind _output_get (Variables|Default|SetActivePlayer _activeplayer))
  (Development|PrintString (Utilities|String|Append "Turn started for : " (Utilities|GetDisplayName _output_get)))
  (Utilities|FlowControl|Sequence
    (:then_0
      (bind _cardhandsize (Default|GetHandPileSize (Variables|Default|GetActivePlayer)))
      (bind _cards (CallFunction|GetCardsfromPile (Math|Integer|Max(Integer) (- 5 _cardhandsize))))
      (Default|AddCardstoHand (Variables|Default|GetActivePlayer) _cards))))

(event Custom|StartGame
  (Development|PrintString "GameStarted")
  (bind _cardpile (CallFunction|GenerateCards 200))
  (Variables|Default|SetCard%20Pile _cardpile)
  (CallFunction|ExecuteTurn))

(event Custom|HandlePlayerEndTurn
  (params (PlayerOwner :type BP%20Tropicalia%20Player%20Object%20Reference) (UsedCards :type Array%20of%20BP%20Card%20Object%20References))
  (Development|PrintString "Player Ended Turn 
================================")
  (CallFunction|UpdateGrid UsedCards)
  (bind _gamehasended (CallFunction|HasGameEnded))
  (switch Utilities|FlowControl|Switch|SwitchonE_GameHasEndedResult _gamehasended
    (:NewEnumerator2
      (CallFunction|ExecuteTurn))
    (:NewEnumerator0
      (Development|PrintString "Won"))
    (:NewEnumerator1
      (Development|PrintString "Lose"))))

(event Custom|HandleAddCardsToHandComplete
  (params (Player :type BP%20Tropicalia%20Player%20Object%20Reference))
  (Development|PrintString "DRAW COMPLETE")
  (CallFunction|StartPlayerTurn Player))

(event EventBeginPlay
  (bind _returnvalue (Game|GetPlayerController 0))
  (Utilities|FlowControl|Sequence
    (:then_0
      (Input|EnableInput _returnvalue)
      (Variables|/Script/Engine.PlayerController|SetbShowMouseCursor _returnvalue true)
      (Variables|/Script/Engine.PlayerController|SetbEnableClickEvents _returnvalue true))
    (:then_1
      (bind _outactors (Actor|GetAllActorsOfClass "/Game/TropicaliaJam/BP_TropicaliaPlayer.BP_TropicaliaPlayer_C"))
      (bind _output_get (Variables|Default|SetPlayers _outactors))
      (for _array_element _output_get
        (EventDispatchers|BindEventtoEndTurn _array_element (EventDispatchers|CreateEvent :!event Custom|HandlePlayerEndTurn))
        (EventDispatchers|AssignDrawComplete _array_element (EventDispatchers|CreateEvent :!event Custom|HandleAddCardsToHandComplete))))
    (:then_2
      (bind _cells (CallFunction|SpawnGrid (Variables|Default|GetGridX) (Variables|Default|GetGridY)))
      (for _array_element_2 _cells
        (EventDispatchers|AssignOnClicked _array_element_2 (delegate Custom|OnClicked_Event))))
    (:then_3
      (Utilities|FlowControl|Delay 1.0)
      (CallFunction|StartGame))))

(event EventTick
  (params (DeltaSeconds :type Float%20%28single-precision%29)))

(fn ConstructionScript)

(fn SpawnGrid
  (params (Columns :type Integer) (Rows :type Integer))
  (bind _cellmesh (LocalVariables|GetCellMesh))
  (bind _padding (LocalVariables|GetPadding))
  (bind _returnvalue (StaticMesh|GetBoundingBox _cellmesh))
  (bind _returnvalue_2 (- (.max _returnvalue) (.min _returnvalue)))
  (bind (_x _y) (Math|Vector|BreakVector _returnvalue_2))
  (Variables|Default|SetGridX Columns)
  (Variables|Default|SetGridY Rows)
  (for _index (range 0 (- Rows 1))
    (for _index_2 (range 0 (- Columns 1))
      (bind _returnvalue_3 (Game|SpawnActorfromClass "/Game/TropicaliaJam/BP_GridCell.BP_GridCell_C" (Math|Transform|MakeTransform (Math|Transform|TransformLocation (Transformation|GetActorTransform) (Math|Vector|MakeVector (* _index_2 (+ _x _padding)) (* _index (+ _y _padding)) 0.0)) "0, 0, 0" (Transformation|GetActorScale3D)) "Undefined" 0 0))
      (Utilities|Array|Add (Variables|Default|GetCells) _returnvalue_3)))
  (return (Variables|Default|GetCells)))

(fn SelectActivePlayer
  (return (Utilities|Array|Get(acopy) (Variables|Default|GetPlayers))))

(fn GetNCardsfromPile
  (params (Number :type Integer))
  (Development|PrintString (Utilities|String|ToString(Text) (Utilities|Text|FormatText "Giving {1} cards to player {2}" Number (Utilities|GetDisplayName (Variables|Default|GetActivePlayer)))))
  (return (Utilities|Array|MakeArray 0 0 0)))

(fn StartPlayerTurn
  (params (Player :type BP%20Tropicalia%20Player%20Object%20Reference))
  (Default|StartTurn Player))

(fn UpdateGrid
  (params (Array :type Array%20of%20BP%20Card%20Object%20References))
  (for _array_element Array
    _))

(fn HasGameEnded
  (if false
    (return "NewEnumerator0")
    (else
      (return "NewEnumerator2"))))

(fn GenerateCards
  (params (Count :type Integer))
  (for _index (range 1 Count)
    (bind _returnvalue (Game|SpawnActorfromClass "/Game/TropicaliaJam/BP_Card.BP_Card_C" (Transformation|GetWorldTransform (Variables|Default|GetCardPilePivot)) "Undefined" 0 (Utilities|Enum|ByteToEnumE_CardType (Math|Conversions|ToByte(Integer) (- (|GetNumEnumEntries) 1))) (Utilities|Enum|ByteToEnumE_CardModifications (Math|Conversions|ToByte(Integer) (- (|GetNumEnumEntries) 1))) "(X=-1.000000,Y=-1.000000)" 0))
    (Utilities|Array|Add (LocalVariables|Getpile) _returnvalue))
  (return (LocalVariables|Getpile)))

(fn GetCardsfromPile
  (params (CardCount :type Integer))
  (bind _card_pile (Variables|Default|GetCard%20Pile))
  (bind _returnvalue (Utilities|Array|LastIndex _card_pile))
  (bind _output (Utilities|Array|Get(acopy) _card_pile _returnvalue))
  (Development|PrintString (Utilities|String|ToString(Text) (Utilities|Text|FormatText "Giving {1} cards to player {2}" 0 (Utilities|GetDisplayName (Variables|Default|GetActivePlayer)))))
  (for _index (range 1 CardCount)
    (if (>= _returnvalue 0)
      (Utilities|Array|Add (LocalVariables|GetReturn) _output)
      (Utilities|Array|RemoveItem _card_pile _output)
      (else
        (return (LocalVariables|GetReturn) true))))
  (return (LocalVariables|GetReturn) (Utilities|Array|IsEmpty (Variables|Default|GetCard%20Pile))))

(fn GetActivePlayer
  (return (Variables|Default|GetActivePlayer)))