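; BP_GridCell is a single cell of the grid, storing a Tension value and displaying it through its static mesh.
; SetTension writes the value into the mesh's custom primitive data at index 0, where a material can read it.
; On BeginPlay it caches its owning BP_Grid.
; Cursor hover queries the active player's selected card through the grid but does nothing with it yet, and hover end is empty.
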(event OnBeginCursorOver(StaticMesh)
  (params (TouchedComponent :type Primitive%20Component%20Object%20Reference))
  (bind _activeplayer (Default|GetActivePlayer (Variables|Default|GetGrid)))
  (Default|GetSelectedCard _activeplayer))

(event OnEndCursorOver(StaticMesh)
  (params (TouchedComponent :type Primitive%20Component%20Object%20Reference)))

(event EventBeginPlay
  (bind _asbp_grid (Utilities|Casting|CastToBP_Grid (Components|GetOwner)))
  (Variables|Default|SetGrid _asbp_grid))

(fn ConstructionScript)

(fn SetTension
  (params (Tension :type Float%20%28double-precision%29))
  (Variables|Default|SetTension Tension)
  (Rendering|Material|SetCustomPrimitiveDataVector4 (Variables|Default|GetStaticMesh) 0 (Math|Vector4|MakeVector4 Tension 0.0 0.0 0.0)))